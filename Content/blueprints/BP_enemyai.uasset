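; Enemy AI character that chases the player on sight and attacks with an axe that knocks characters back.
; Pawn sensing triggers an AI MoveTo toward the player, which on arrival plays the attack montage with a whoosh sound, gated by a CanAttack flag until the montage ends.
; A montage notify fires a forward sphere trace that launches any hit Character forward and up, with an impact sound.
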(event `self.ReceiveBeginPlay`)

(event `chase player`
  (bind _returnvalue (`self.K2_GetActorLocation`))
  (`|AIMoveTo` self (0.0 0.0 0.0) (`GameplayStatics.GetPlayerCharacter` 0) 80.0
    (:`OnSuccess`
      (if (`self.CanAttack?`)
        (`|PlayMontage` (`self.Mesh`) "/Game/Characters/villager/Your_First_Game_2025_Masterclass_Resources/2025_Masterclass_Resources/PlayerCharacter/animation/attack/a-attack-montoge.a-attack-montoge"
          (:`then`
            (set `self.CanAttack?` false)
            (`GameplayStatics.PlaySoundAtLocation` "/Game/Audio/MS_AxeWoosh.MS_AxeWoosh" (`self.K2_GetActorLocation`) (struct) 1.0 1.0 0.0 null null null null))
          (:`OnCompleted`
            (set `self.CanAttack?` true :!label _label))
          (:`OnInterrupted`
            (goto _label))
          (:`OnNotifyBegin`
            (bind (_outhit _returnvalue_2) (`KismetSystemLibrary.SphereTraceSingle` :`Start` _returnvalue :`End` (+ _returnvalue (* (`KismetMathLibrary.GetForwardVector` (`self.K2_GetActorRotation`)) 180.0)) :`TraceChannel` "TraceTypeQuery3" :`DrawTime` 0.5))
            (if _returnvalue_2
              (bind _ascharacter (cast `Character` (`.HitActor` (`GameplayStatics.BreakHitResult` _outhit))))
              (`self.LaunchCharacter` _ascharacter (+ (* (`KismetMathLibrary.GetForwardVector` (`self.K2_GetActorRotation`)) (`self.frontknockbar`)) (`KismetMathLibrary.MakeVector` 0.0 0.0 (`self.upwards knockback`))) false false)
              (`GameplayStatics.PlaySoundAtLocation` "/Game/Audio/MS_AxeHit.MS_AxeHit" (`self.K2_GetActorLocation`) (struct) 1.0 1.0 0.0 null null null null))))))))

(event `self.PawnSensing.OnSeePawn`
  (params (Pawn :type "Pawn Object Reference"))
  (`self.chase player`))

(fn `UserConstructionScript`)